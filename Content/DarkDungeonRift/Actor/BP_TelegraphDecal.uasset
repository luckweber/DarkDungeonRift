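; BP_TelegraphDecal is a self-destroying decal actor that shows a timed, filling telegraph shape.
; On BeginPlay it sizes the decal from Radius, with an optional width override, then creates a dynamic material instance fed with color and cone half-angle.
; A timeline, rate-scaled to match Duration, drives the material's Fill parameter.
; When the fill finishes, the actor waits ExtraLifetime and then destroys itself.
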(event `self.ReceiveBeginPlay`
  (bind _decal (`self.Decal`))
  (`DecalComponent.SetDecalMaterial` _decal (`self.DecalMaterial`))
  (`SceneComponent.SetRelativeScale3D` _decal (`KismetMathLibrary.MakeVector` 10.0 (select `bool` (> (`self.WidthOverride`) 0.0) :`false` (`self.Radius`) :`true` (`self.WidthOverride`)) (`self.Radius`)))
  (bind _returnvalue (`DecalComponent.CreateDynamicMaterialInstance` _decal))
  (bind _output_get (set `self.MID` _returnvalue))
  (`MaterialInstanceDynamic.SetVectorParameterValue` _output_get "Color" (`self.Color`))
  (`MaterialInstanceDynamic.SetScalarParameterValue` (`self.MID`) "ConeHalfAngleDeg" (`self.ConeHalfAngleDeg`))
  (`TimelineComponent.SetPlayRate` (`self.Timeline FillTL`) (/ 1.0 (`KismetMathLibrary.FMax` (`self.Duration`) 0.05)))
  (bind (_direction _alpha) (`Timeline|Timeline FillTL`)
    (:`Update`
      (`MaterialInstanceDynamic.SetScalarParameterValue` (`self.MID`) "Fill" _alpha))
    (:`Finished`
      (`KismetSystemLibrary.Delay` (`self.ExtraLifetime`))
      (`self.K2_DestroyActor`))))

(fn `UserConstructionScript`)